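; BP_Checkpoint is a collectible checkpoint that awards points to BP_Crow and triggers its win when it is the last one left.
; A sphere overlap by the crow plays a sound, adds PointValue to the score, checks for a win, then fades out.
; CheckForWin counts remaining BP_Checkpoint actors, including itself.
; Fade drives the material's OpacityValue with a timeline and destroys the actor only when finished.
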(event `self.SphereCollision.OnComponentBeginOverlap`
  (params (OverlappedComponent :type "PrimitiveComponent Object Reference") (OtherActor :type "Actor Object Reference") (OtherComp :type "PrimitiveComponent Object Reference") (OtherBodyIndex :type Integer) (bFromSweep :type Boolean) (SweepResult :type "HitResult Structure (by ref)"))
  (bind _asbp_crow (cast `/Game/Blueprints/BP_Crow` OtherActor))
  (`|ExecutionSequence`
    (:`then_0`
      (`GameplayStatics.PlaySound2D` "/Game/SFX/good_checkpoint.good_checkpoint" 1.0 1.0 0.0 null null))
    (:`then_1`
      (`/Game/Blueprints/BP_Crow.AddToScore` _asbp_crow (`self.PointValue`)))
    (:`then_2`
      (bind _iswin (`self.CheckForWin`))
      (if _iswin
        (`/Game/Blueprints/BP_Crow.Win` _asbp_crow)))
    (:`then_3`
      (bind (_direction _newtrack_0) (`Timeline|Timeline` :!via `PlayFromStart`)
        (:`Update`
          (`MeshComponent.SetScalarParameterValueOnMaterials` (`self.Sphere`) "OpacityValue" _newtrack_0))
        (:`Finished`
          (`self.K2_DestroyActor`))))))

(fn `CheckForWin`
  (returns (IsWin :type Boolean))
  (bind _outactors (`GameplayStatics.GetAllActorsOfClass` "BP_Checkpoint_C"))
  (return (== (`KismetArrayLibrary.Array_Length` _outactors) 1)))

(fn `UserConstructionScript`)